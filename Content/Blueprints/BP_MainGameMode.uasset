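; BP_MainGameMode is a game mode Blueprint that sets up input for gameplay when play begins.
; On BeginPlay it hides the first player controller's cursor, disables click and mouse-over events, focuses the viewport and switches to game-only input.
; Its TogglePause override defers to the parent implementation, followed by a paused-state check with no actions attached.
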(event EventBeginPlay
  (bind _returnvalue (Game|GetPlayerController 0))
  (Variables|/Script/Engine.PlayerController|SetbShowMouseCursor _returnvalue false)
  (Variables|/Script/Engine.PlayerController|SetbEnableClickEvents _returnvalue false)
  (Variables|/Script/Engine.PlayerController|SetbEnableMouseOverEvents _returnvalue false)
  (Class|WidgetBlueprintLibrary|SetFocustoGameViewport)
  (Input|SetInputModeGameOnly (Game|GetPlayerController 0) false))

(event EventTick
  (params (DeltaSeconds :type Float%20%28single-precision%29)))

(event EventTogglePause
  (params (PlayerController :type Player%20Controller%20Object%20Reference))
  ;[1 1 1] Pause menu toggle
  (|CallParentFunction PlayerController)
  (if (Game|IsGamePaused)
    _))

(fn ConstructionScript)