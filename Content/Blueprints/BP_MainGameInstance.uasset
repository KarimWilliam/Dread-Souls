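; Game instance Blueprint that applies master, dialogue, effects and music volume changes to the game's audio buses.
; Each volume event calls its parent implementation, then passes the value to BusSetVolume.
; Master and dialogue each drive one bus, while effects covers generic sounds and Foley.
; The music setting controls the internal and external ambience buses.
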(event EventChangeMasterVolume
  (params (Value :type Float%20%28single-precision%29))
  (|CallParentFunction Value)
  (Class|FMODBlueprintStatics|BusSetVolume "/Game/FMOD/Buses/UnrealMasterBus.UnrealMasterBus" Value))

(event EventChangeDialogueVolume
  (params (Value :type Float%20%28single-precision%29))
  (|CallParentFunction Value)
  (Class|FMODBlueprintStatics|BusSetVolume "/Game/FMOD/Buses/UnrealMasterBus/DialogueSFX.DialogueSFX" Value))

(event EventChangeEffectsVolume
  (params (Value :type Float%20%28single-precision%29))
  (|CallParentFunction Value)
  (Class|FMODBlueprintStatics|BusSetVolume "/Game/FMOD/Buses/UnrealMasterBus/GenericSounds.GenericSounds" Value)
  (Class|FMODBlueprintStatics|BusSetVolume "/Game/FMOD/Buses/UnrealMasterBus/foley.foley" Value))

(event EventChangeMusicVolume
  (params (Value :type Float%20%28single-precision%29))
  (|CallParentFunction Value)
  (Class|FMODBlueprintStatics|BusSetVolume "/Game/FMOD/Buses/UnrealMasterBus/AmbienceInternal.AmbienceInternal" Value)
  (Class|FMODBlueprintStatics|BusSetVolume "/Game/FMOD/Buses/UnrealMasterBus/AmbienceExternal.AmbienceExternal" Value))