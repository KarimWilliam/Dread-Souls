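; Main player character Blueprint that adds spawn, hit feedback and turning presentation on top of an action-component-driven parent.
; BeginPlay starts SpawnAction and runs a two-stage camera fade in from black.
; GetHit calls the parent, then plays a world camera shake at the impact point.
; An interruptible timeline lerps capsule rotation for 180-degree turns and stops TurnAction on finish; leftover debug nodes are disconnected.
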(event Custom|180Turn
  ;[1 1 1 1 34] Turning Timeline and logic
  (bind _turntrack (Timeline|180TurnTimeline PlayFromStart)
    (:Update
      (Transformation|SetWorldRotation (Variables|Default|GetCapsuleComponent) (Math|Rotator|Lerp(Rotator) (Math|Conversions|RotationFromXVector (Variables|Default|GetStartRotation)) (Math|Conversions|RotationFromXVector (Variables|Default|GetEndRotation)) _turntrack) false false))
    (:Finished
      (Class|ActionComponent|StopActionbyName (Variables|Default|GetActionComp) 0 "TurnAction"))))

(event Custom|Interrupt%20180Turn
  ;[1 1 1 1 34] Turning Timeline and logic
  (bind _turntrack (Timeline|180TurnTimeline Stop)
    (:Update
      (Transformation|SetWorldRotation (Variables|Default|GetCapsuleComponent) (Math|Rotator|Lerp(Rotator) (Math|Conversions|RotationFromXVector (Variables|Default|GetStartRotation)) (Math|Conversions|RotationFromXVector (Variables|Default|GetEndRotation)) _turntrack) false false))
    (:Finished
      (Class|ActionComponent|StopActionbyName (Variables|Default|GetActionComp) 0 "TurnAction"))))

(event EventTick
  (params (DeltaSeconds :type Float%20%28single-precision%29)))

(event EventBeginPlay
  (bind _returnvalue (Game|GetPlayerCameraManager 0))
  ;[1 1 1 1 40] BeginPlay
  (Class|ActionComponent|StartActionbyName (Variables|Default|GetActionComp) self "SpawnAction")
  (CameraFades|StartCameraFade _returnvalue 1.0 0.8 1.0 "(R=0.000000,G=0.000000,B=0.000000,A=1.000000)" true true)
  (Utilities|FlowControl|Delay 1.0)
  (CameraFades|StartCameraFade _returnvalue 0.8 0.0 2.0 "(R=0.000000,G=0.000000,B=0.000000,A=1.000000)" true false))

(event EventGetHit
  (params (ImpactPoint :type Vector%20%28by%20ref%29 :default "0, 0, 0") (Hitter :type Actor%20Object%20Reference) (CauseStagger :type Boolean))
  ;[1 1 1 1 40] Camera Shake
  (|CallParentFunction ImpactPoint Hitter CauseStagger)
  (Camera|PlayWorldCameraShake "/Game/Blueprints/Misc/MainGetHitCameraShake.MainGetHitCameraShake_C" ImpactPoint 0.0 5e+02 0.0))

(fn ConstructionScript)

(fn PrintActiveGameplayTags
  (for _array_element (GameplayTags|BreakGameplayTagContainer (Variables|/Script/StylizedTest.ActionComponent|GetActiveGamePlayTags (Variables|Default|GetActionComp)))
    (Development|PrintString (GameplayTags|GetDebugStringfromGameplayTag _array_element))))