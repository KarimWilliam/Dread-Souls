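; BossWalkAura is an aura actor, named for a boss, that temporarily disrupts the main character's controls and movement speed on contact.
; Sphere overlap with MainCharacter removes the IMC_Main Enhanced Input context from player 0 and sets walk speed to the character's HealMoveSpeed.
; After a five-second Delay, it sets speed to RunSpeed, re-adds the mapping context and destroys itself.
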(event OnComponentBeginOverlap(Sphere)
  (params (OverlappedComponent :type Primitive%20Component%20Object%20Reference) (OtherActor :type Actor%20Object%20Reference) (OtherComp :type Primitive%20Component%20Object%20Reference) (OtherBodyIndex :type Integer) (bFromSweep :type Boolean) (SweepResult :type Hit%20Result%20Structure%20%28by%20ref%29))
  (bind _returnvalue (Game|GetPlayerController 0))
  (bind _returnvalue_2 (PlayerController|LocalPlayerSubsystems|GetEnhancedInputLocalPlayerSubsystem _returnvalue))
  (bind _asmain_character (Utilities|Casting|CastToMainCharacter OtherActor))
  (Input|RemoveMappingContext _returnvalue_2 "/Game/Inputs/IMC_Main.IMC_Main" "(bIgnoreAllPressedKeysUntilRelease=True,bForceImmediately=False)")
  (Variables|/Script/Engine.CharacterMovementComponent|SetMaxWalkSpeed (Variables|/Script/Engine.Character|GetCharacterMovement _asmain_character) (Variables|/Script/StylizedTest.BaseCharacter|GetHealMoveSpeed _asmain_character))
  (Utilities|FlowControl|Delay 5.0)
  (Variables|/Script/Engine.CharacterMovementComponent|SetMaxWalkSpeed (Variables|/Script/Engine.Character|GetCharacterMovement _asmain_character) (Variables|/Script/StylizedTest.BaseCharacter|GetRunSpeed _asmain_character))
  (Input|AddMappingContext _returnvalue_2 "/Game/Inputs/IMC_Main.IMC_Main" 0 "(bIgnoreAllPressedKeysUntilRelease=True,bForceImmediately=False)")
  (Actor|DestroyActor))

(event EventBeginPlay)

(event Collision|EventActorBeginOverlap
  (params (OtherActor :type Actor%20Object%20Reference)))

(event EventTick
  (params (DeltaSeconds :type Float%20%28single-precision%29)))

(fn ConstructionScript)